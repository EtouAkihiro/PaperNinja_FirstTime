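; PNGearActor is a gear actor with up to four gear meshes that spins around its yaw axis.
; The Construction Script uses a DestroyGear helper to remove each mesh component whose Gear01–Gear04 flag is off, so each instance chooses its visible gears.
; On BeginPlay, it sets the RotatingMovement yaw rate from RotationSpeed, negated when IsReverse is true.
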(event `self.ReceiveBeginPlay`
  (set `RotatingMovementComponent.RotationRate` (`KismetMathLibrary.MakeRot` 0.0 (* (`self.RotationSpeed`) (`KismetMathLibrary.SelectFloat` -1.0 1.0 (`self.IsReverse`)))) (`self.RotatingMovement`)))

(event `self.ReceiveActorBeginOverlap`
  (params (OtherActor :type "Actor Object Reference")))

(event `self.ReceiveTick`
  (params (DeltaSeconds :type "Float (single-precision)")))

(fn `DestroyGear`
  (params (Condition :type Boolean) (Component :type "ActorComponent Object Reference"))
  (if (not Condition)
    (`ActorComponent.K2_DestroyComponent` Component))
  (return))

(fn `UserConstructionScript`
  (`self.DestroyGear` (`self.Gear01`) (`self.GearMesh01`))
  (`self.DestroyGear` (`self.Gear02`) (`self.GearMesh02`))
  (`self.DestroyGear` (`self.Gear03`) (`self.GearMesh03`))
  (`self.DestroyGear` (`self.Gear04`) (`self.GearMesh04`)))
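; Player controller that routes look and movement input through a custom PNPlayerCameraManager, cached on BeginPlay.
; Look axes feed yaw and pitch into the camera manager, while move axes drive the controlled pawn along the camera's flattened forward and right vectors.
; When notified of an obtained scroll, it disables camera control, sets a desired rotation relative to the pawn's facing, then narrows the desired FOV after a short delay.
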(event `self.ReceiveBeginPlay`
  (bind _aspnplayer_camera_manager (cast `/Game/Blueprints/PNPlayerCameraManager` (`GameplayStatics.GetPlayerCameraManager` 0)))
  (set `self.MyCameraManager` _aspnplayer_camera_manager))

(event `self.ReceiveTick`
  (params (DeltaSeconds :type "Float (single-precision)")))

(event `InputAxis|LookRight`
  (params (AxisValue :type "Float (single-precision)"))
  (`/Game/Blueprints/PNPlayerCameraManager.AddYawInput` (`self.MyCameraManager`) AxisValue))

(event `InputAxis|LookUp`
  (params (AxisValue :type "Float (single-precision)"))
  (`/Game/Blueprints/PNPlayerCameraManager.AddPitchInput` (`self.MyCameraManager`) AxisValue))

(event `InputAxis|MoveForward`
  (params (AxisValue :type "Float (single-precision)"))
  (`Pawn.AddMovementInput` (`self.K2_GetPawn`) (`/Game/Blueprints/PNFuncLibrary.FlattenDirection` (`/Game/Blueprints/PNPlayerCameraManager.GetCameraForwardVector` (`self.MyCameraManager`))) AxisValue false))

(event `InputAxis|MoveRight`
  (params (AxisValue :type "Float (single-precision)"))
  (`Pawn.AddMovementInput` (`self.K2_GetPawn`) (`/Game/Blueprints/PNFuncLibrary.FlattenDirection` (`/Game/Blueprints/PNPlayerCameraManager.GetCameraRightVector` (`self.MyCameraManager`))) AxisValue false))

(event `NotifyObtainedScroll`
  (bind _mycameramanager (`self.MyCameraManager`))
  (set `/Game/Blueprints/PNPlayerCameraManager.Is Enable Control` false _mycameramanager)
  (set `/Game/Blueprints/PNPlayerCameraManager.DesiredRotation` (`KismetMathLibrary.MakeRot` 20.0 (- (.yaw (`self.K2_GetActorRotation` (`self.K2_GetPawn`))) 15.0) (.roll (`self.K2_GetActorRotation` (`self.K2_GetPawn`)))) _mycameramanager)
  (`KismetSystemLibrary.Delay` 1.0)
  (set `/Game/Blueprints/PNPlayerCameraManager.DesiredFOV` 30.0 _mycameramanager))

(fn `PMPlayerCameraManager`
  (returns (ReturnValue :type "/Game/Blueprints/PNPlayerCameraManager Object Reference"))
  (return (`self.MyCameraManager`)))

(fn `UserConstructionScript`)
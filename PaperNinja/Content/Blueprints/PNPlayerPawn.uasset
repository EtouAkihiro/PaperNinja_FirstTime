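; Player character with camera-relative movement, look and sprint, carrying coins and able to obtain the goal scroll.
; A looping timer drops a coin while flat speed reaches sprint speed, launching it as a physics pickup in a random direction.
; The first damage is fatal: it ragdolls the mesh, scatters all coins, plays death effects and switches BGM through PNGameMode.
; Obtaining the scroll stops movement and later switches BGM.
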(event `self.ReceiveTick`
  (params (DeltaSeconds :type "Float (single-precision)")))

(event `self.ReceiveActorBeginOverlap`
  (params (OtherActor :type "Actor Object Reference")))

(event `self.ReceiveBeginPlay`
  (set `CharacterMovementComponent.MaxWalkSpeed` (`self.Ground Walk Speed`) (`self.CharacterMovement`))
  (`KismetSystemLibrary.K2_SetTimer` null "CheckSprintRisk" 0.5 true))

(event `InputAxis|MoveForward`
  (params (AxisValue :type "Float (single-precision)"))
  (`self.AddMovementInput` (`self.FlattenDirection` (`SceneComponent.GetForwardVector` (`self.Camera`))) AxisValue) ; 前進
)

(event `InputAxis|MoveRight`
  (params (AxisValue :type "Float (single-precision)"))
  (`self.AddMovementInput` (`self.FlattenDirection` (`SceneComponent.GetRightVector` (`self.Camera`))) AxisValue))

(event `InputAction|sPRINT`
  (bind _charactermovement (`self.CharacterMovement`))
  (:`Pressed`
    (set `CharacterMovementComponent.MaxWalkSpeed` (`self.GroundSprintSpeed`) _charactermovement))
  (:`Released`
    (set `CharacterMovementComponent.MaxWalkSpeed` (`self.Ground Walk Speed`) _charactermovement)))

(event `InputAxis|LookUp`
  (params (AxisValue :type "Float (single-precision)"))
  (`self.AddControllerPitchInput` AxisValue))

(event `InputAxis|LookRight`
  (params (AxisValue :type "Float (single-precision)"))
  (`self.AddControllerYawInput` AxisValue))

(event `self.ReceiveAnyDamage`
  (params (Damage :type "Float (single-precision)") (DamageType :type "DamageType Object Reference") (InstigatedBy :type "Controller Object Reference") (DamageCauser :type "Actor Object Reference"))
  (bind _mesh (`self.Mesh`))
  (`/Engine/EditorBlueprintResources/StandardMacros.DoOnce` false
    (:`Completed`
      (`|ExecutionSequence`
        (:`then_0`
          (`KismetSystemLibrary.PrintString` "Died!")
          (`CharacterMovementComponent.DisableMovement` (`self.CharacterMovement`))
          (`self.SetLifeSpan` 5.0)
          (`PrimitiveComponent.SetCollisionProfileName` _mesh "Ragdoll")
          (`PrimitiveComponent.SetSimulatePhysics` _mesh true)
          (`PrimitiveComponent.SetCollisionProfileName` (`self.CapsuleComponent`) "Spectator"))
        (:`then_1`
          (`self.DropAllCoins`))
        (:`then_2`
          (`ActorComponent.Activate` (`self.DeathFX`) false)
          (`GameplayStatics.PlaySoundAtLocation` "/Game/Audio/player_death_Cue.player_death_Cue" (`self.K2_GetActorLocation`)) ; 死亡音を発音する
          (`KismetSystemLibrary.Delay` 1.0)
          (`/Game/Blueprints/PNGameMode.PlayBGM` (cast `/Game/Blueprints/PNGameMode` (`GameplayStatics.GetGameMode`) :!pure true) "/Game/Audio/bgm03_Cue.bgm03_Cue"))))))

(event `ObtainScroll`
  (`CharacterMovementComponent.DisableMovement` (`self.CharacterMovement`)) ; キャラの動きを止める
  (set `self.HasScroll` true)
  (`KismetSystemLibrary.Delay` 5.0)
  (`KismetSystemLibrary.PrintString` "Goal")
  (`/Game/Blueprints/PNGameMode.PlayBGM` (cast `/Game/Blueprints/PNGameMode` (`GameplayStatics.GetGameMode`) :!pure true) "/Game/Audio/bgm03_Cue.bgm03_Cue"))

(event `DropAllCoins`
  (while (> (`self.NumOfCoins`) 0)
    (`self.DropCoin`)))

(fn `AddCoin`
  (params (Num :type Integer :default 0))
  (set `self.NumOfCoins` (+ (`self.NumOfCoins`) Num)))

(fn `CheckSprintRisk`
  (if (>= (`/Game/Blueprints/PNActorMacroLibrary.GetFlatSpeed`) (`self.GroundSprintSpeed`))
    (`self.DropCoin`)))

(fn `DropCoin`
  (if (>= (`self.NumOfCoins`) 1)
    (set `self.NumOfCoins` (- (`self.NumOfCoins`) 1))
    (bind _returnvalue (`|SpawnActorFromClass` "/Game/Blueprints/PNPickupCoinActor.PNPickupCoinActor_C" (`SceneComponent.GetSocketTransform` (`self.Mesh`) "CoinSpawnPoint" "RTS_World")))
    (`PrimitiveComponent.SetSimulatePhysics` _returnvalue true)
    (`PrimitiveComponent.AddImpulse` _returnvalue (`KismetMathLibrary.RotateAngleAxis` (`KismetMathLibrary.MakeVector` 200.0 0.0 200.0) (`KismetMathLibrary.RandomFloatInRange` 0.0 360.0) (0.0 0.0 1.0)) "None" true)))

(fn `FlattenDirection`
  (params (In :type "Object.Vector Structure" :default (0.0 0.0 0.0)))
  (returns (RetumValue :type "Object.Vector Structure"))
  (return (`KismetMathLibrary.Normal` (`/Game/Blueprints/PNFuncLibrary.Flatten Vector` In))))

(fn `GetNumOfCoins`
  (returns (ReturnValue :type Integer))
  (return (`self.NumOfCoins`)))

(fn `UserConstructionScript`)
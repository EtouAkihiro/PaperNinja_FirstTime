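; PNSwitchActor is a pressure switch that sinks its mesh and signals on or off when something overlaps its trigger box.
; A timeline lerps the mesh down; on finishing in either direction it calls OnTurnedOn or OnTurnedOff and tints the dynamic material green or red.
; Momentary switches reverse when an overlap ends, while others stay pressed until the TrunOff event reverses them.
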(event `self.ReceiveBeginPlay`
  (bind _mesh (`self.Mesh`))
  (bind _returnvalue (`PrimitiveComponent.CreateDynamicMaterialInstance` _mesh 0 (`PrimitiveComponent.GetMaterial` _mesh 0)))
  (bind _output_get (set `self.MeshIMD` _returnvalue))
  (`MaterialInstanceDynamic.SetVectorParameterValue` _output_get "Tint Base Color" (struct :`R` 1.0 :`A` 1.0)))

(event `self.BoxTigger.OnComponentBeginOverlap`
  (params (OtherActor :type "Actor Object Reference") (OtherComp :type "PrimitiveComponent Object Reference") (OtherBodyIndex :type Integer) (bFromSweep :type Boolean) (SweepResult :type "EngineTypes.HitResult Structure (by ref)"))
  (bind _meshimd (`self.MeshIMD`))
  (bind (_direction _alpha) (`Timeline|SwitchTimeline` :!label _label)
    (:`Update`
      (`SceneComponent.K2_SetRelativeLocation` (`self.Mesh`) (`KismetMathLibrary.VLerp` (0.0 0.0 0.0) (0.0 0.0 -8.0) _alpha) false))
    (:`Finished`
      (switch `TimelineComponent.ETimelineDirection` _direction
        (:`Forward`
          (`self.OnTurnedOn`)
          (`MaterialInstanceDynamic.SetVectorParameterValue` _meshimd "Tint Base Color" (struct :`G` 1.0 :`A` 1.0)))
        (:`Backward`
          (`self.OnTurnedOff`)
          (`MaterialInstanceDynamic.SetVectorParameterValue` _meshimd "Tint Base Color" (struct :`R` 1.0 :`A` 1.0)))))))

(event `self.BoxTigger.OnComponentEndOverlap`
  (params (OtherActor :type "Actor Object Reference") (OtherComp :type "PrimitiveComponent Object Reference") (OtherBodyIndex :type Integer))
  (if (`self.Is Momentary`)
    (goto _label :!via `Reverse`)))

(event `TrunOff`
  (goto _label :!via `Reverse`))

(event `self.ReceiveActorBeginOverlap`
  (params (OtherActor :type "Actor Object Reference")))

(event `self.ReceiveTick`
  (params (DeltaSeconds :type "Float (single-precision)")))

(fn `UserConstructionScript`)
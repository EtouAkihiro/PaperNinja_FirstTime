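; Shuriken projectile actor that flies through the world, bouncing off what it hits and damaging actors it overlaps.
; On BeginPlay it rotates its initial velocity by the actor's rotation and scales it by Speed.
; Tick moves it manually with a swept location update, without using a projectile movement component.
; Hits mirror the velocity around a flattened surface normal, and overlaps apply fixed damage without destroying the shuriken.
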(event `self.ReceiveActorBeginOverlap`
  (params (OtherActor :type "Actor Object Reference"))
  (`GameplayStatics.ApplyDamage` OtherActor 100.0))

(event `self.ReceiveTick`
  (params (DeltaSeconds :type "Float (single-precision)"))
  (`self.K2_SetActorLocation` (+ (`self.K2_GetActorLocation`) (* (`self.WorldVelocity`) DeltaSeconds)) true))

(event `self.ReceiveBeginPlay`
  (set `self.WorldVelocity` (* (`KismetMathLibrary.GreaterGreater_VectorRotator` (`self.WorldVelocity`) (`self.K2_GetActorRotation`)) (`self.Speed`))))

(event `self.ReceiveHit`
  (params (MyComp :type "PrimitiveComponent Object Reference") (Other :type "Actor Object Reference") (OtherComp :type "PrimitiveComponent Object Reference") (bSelfMoved :type Boolean) (HitLocation :type "Object.Vector Structure") (HitNormal :type "Object.Vector Structure") (NormalImpulse :type "Object.Vector Structure") (Hit :type "EngineTypes.HitResult Structure (by ref)"))
  (set `self.WorldVelocity` (`KismetMathLibrary.MirrorVectorByNormal` (`self.WorldVelocity`) (`/Game/Blueprints/PNFuncLibrary.FlattenDirection` HitNormal))))

(fn `UserConstructionScript`)